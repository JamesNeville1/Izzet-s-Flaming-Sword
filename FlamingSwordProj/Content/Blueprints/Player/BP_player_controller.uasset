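; Player controller that spawns and possesses the player character, adds the player's Enhanced Input mapping context and creates the player HUD widget.
; Setup runs in a Start event, which also calls Start on the new character.
; Input actions for movement, look, jump, sprint, inspect, default attack and ranged attack are forwarded to the player character as interface messages, keeping gameplay logic out of the controller.
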(event Custom|Start
  (bind _returnvalue (Game|SpawnActorfromClass "/Game/Blueprints/Player/BP_player.BP_player_C" (Math|Transform|MakeTransform "0.000000,0.000000,50.000000") "Undefined" "MultiplyWithRoot" 0 0))
  (Pawn|Possess _returnvalue)
  (Input|AddMappingContext (PlayerController|LocalPlayerSubsystems|GetEnhancedInputLocalPlayerSubsystem self) "/Game/Blueprints/Input/IMC_player.IMC_player" 0 "(bIgnoreAllPressedKeysUntilRelease=True,bForceImmediately=False)")
  (Default|Start _returnvalue)
  (bind _returnvalue_2 (UserInterface|CreateWidget "/Game/Blueprints/UI/BP_player_ui.BP_player_ui_C" (Game|GetPlayerController 0)))
  (UserInterface|Viewport|AddtoViewport _returnvalue_2 0))

(event Input|EnhancedActionEvents|EnhancedInputActionIA_player_movement
  (params (ActionValue :type Vector%202D%20Structure) (ElapsedSeconds :type Float%20%28double-precision%29) (TriggeredSeconds :type Float%20%28double-precision%29) (InputAction :type Input%20Action%20Object%20Reference :default "/Game/Blueprints/Input/IA_player_movement.IA_player_movement"))
  (bind _returnvalue (Game|GetPlayerCharacter 0))
  (:Triggered
    (Class|BPIPlayerInput|IAPlayerMovement(Message) _returnvalue (.x ActionValue) (.y ActionValue)))
  (:Completed
    (Class|BPIPlayerInput|IAPlayerMovement-End(Message) _returnvalue)))

(event Input|EnhancedActionEvents|EnhancedInputActionIA_player_jump
  (params (ActionValue :type Boolean) (ElapsedSeconds :type Float%20%28double-precision%29) (TriggeredSeconds :type Float%20%28double-precision%29) (InputAction :type Input%20Action%20Object%20Reference :default "/Game/Blueprints/Input/IA_player_jump.IA_player_jump"))
  (bind _returnvalue (Game|GetPlayerCharacter 0))
  (:Triggered
    (Class|BPIPlayerInput|IAPlayerJump(Message) _returnvalue))
  (:Completed
    (Class|BPIPlayerInput|IAPlayerJump-End(Message) _returnvalue)))

(event Input|EnhancedActionEvents|EnhancedInputActionIA_player_sprint
  (params (ActionValue :type Boolean) (ElapsedSeconds :type Float%20%28double-precision%29) (TriggeredSeconds :type Float%20%28double-precision%29) (InputAction :type Input%20Action%20Object%20Reference :default "/Game/Blueprints/Input/IA_player_sprint.IA_player_sprint"))
  (bind _returnvalue (Game|GetPlayerCharacter 0))
  (:Started
    (Class|BPIPlayerInput|IAPlayerSprint-Start(Message) _returnvalue))
  (:Completed
    (Class|BPIPlayerInput|IAPlayerSprint-End(Message) _returnvalue)))

(event Input|EnhancedActionEvents|EnhancedInputActionIA_player_look
  (params (ActionValue :type Vector%202D%20Structure) (ElapsedSeconds :type Float%20%28double-precision%29) (TriggeredSeconds :type Float%20%28double-precision%29) (InputAction :type Input%20Action%20Object%20Reference :default "/Game/Blueprints/Input/IA_player_look.IA_player_look"))
  (:Triggered
    (Class|BPIPlayerInput|IAPlayerLook(Message) (Game|GetPlayerCharacter 0) (.x ActionValue) (.y ActionValue))))

(event Input|EnhancedActionEvents|EnhancedInputActionIA_player_inspect
  (params (ActionValue :type Boolean) (ElapsedSeconds :type Float%20%28double-precision%29) (TriggeredSeconds :type Float%20%28double-precision%29) (InputAction :type Input%20Action%20Object%20Reference :default "/Game/Blueprints/Input/IA_player_inspect.IA_player_inspect"))
  (:Started
    (Class|BPIPlayerInput|IAPlayerInspect-Start(Message) (Game|GetPlayerCharacter 0))))

(event Input|EnhancedActionEvents|EnhancedInputActionIA_player_default_attack
  (params (ActionValue :type Boolean) (ElapsedSeconds :type Float%20%28double-precision%29) (TriggeredSeconds :type Float%20%28double-precision%29) (InputAction :type Input%20Action%20Object%20Reference :default "/Game/Blueprints/Input/IA_player_default_attack.IA_player_default_attack"))
  (:Started
    (Class|BPIPlayerInput|IAPlayerDefaultAttack-Start(Message) (Game|GetPlayerCharacter 0))))

(event Input|EnhancedActionEvents|EnhancedInputActionIA_player_ranged_attack
  (params (ActionValue :type Boolean) (ElapsedSeconds :type Float%20%28double-precision%29) (TriggeredSeconds :type Float%20%28double-precision%29) (InputAction :type Input%20Action%20Object%20Reference :default "/Game/Blueprints/Input/IA_player_ranged_attack.IA_player_ranged_attack"))
  (:Started
    (Class|BPIPlayerInput|IAPlayerRangedAttack-Start(Message) (Game|GetPlayerCharacter 0))))

(fn ConstructionScript)