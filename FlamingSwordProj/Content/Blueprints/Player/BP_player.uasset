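; First-person player character with a flaming sword, handling movement, look, jump, inspect, melee and ranged attacks.
; The head bone is hidden and HeadHook follows the neck for a visible-body view, while direction, speed and torso aim feed the AnimInstance.
; Montage notifies drive the melee combo window and projectile spawn, with timed cooldowns.
; A toggled capsule overlap deals melee damage (trace-timer setup is disconnected), and Tick orients flame gravity.
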(event OnComponentBeginOverlap(Capsule)
  (params (OverlappedComponent :type Primitive%20Component%20Object%20Reference) (OtherActor :type Actor%20Object%20Reference) (OtherComp :type Primitive%20Component%20Object%20Reference) (OtherBodyIndex :type Integer) (bFromSweep :type Boolean) (SweepResult :type Hit%20Result%20Structure%20%28by%20ref%29))
  ;[1 1 1] Default Attack
  (Game|Damage|ApplyDamage OtherActor 1.0 0 0)
  (Development|PrintString (Utilities|GetDisplayName OtherActor)))

(event Custom|Start
  ;[0.6958 1 0.8071] Start
  (Components|SkinnedMesh|HideBonebyName (Variables|Character|GetMesh) "head" "PBO_None")
  (Components|Activation|SetActive (Variables|Default|GetCapsule) false false))

(event Custom|Disable%20Default%20Melee%20Attack%20Cooldown
  ;[1 1 1] Default Attack
  (Variables|DefaultMeleeAttack|SetdefaultMeleeCooldown false))

(event Custom|Default%20Melee%20Attack%20Check
  (bind _hit (CallFunction|AttackCheckRay 1.0))
  (Game|Damage|ApplyDamage _hit 1.0 0 0))

(event Custom|Spawn%20Ranged%20Projectile
  ;[1 1 1] Ranged Attack
  (Game|SpawnActorfromClass "/Game/Blueprints/Player/BP_flame_projectile.BP_flame_projectile_C" (Math|Transform|MakeTransform (Transformation|GetWorldLocation (Variables|Default|GetSM_Prop_Sword_01)) (Utilities|GetRangedProjectileOrientation)) "Undefined" "MultiplyWithRoot" 0 0))

(event Custom|Ranged%20Attack%20Cooldown%20End
  ;[1 1 1] Ranged Attack
  (Variables|RangedMeleeAttack|SetrangedAttackCooldown false))

(event EventEnableDefaultMeleeAttackCooldown
  ;[1 1 1] Default Attack
  (Variables|DefaultMeleeAttack|SetdefaultMeleeCooldown true)
  (Utilities|Time|SetTimerbyEvent (delegate Custom|Disable%20Default%20Melee%20Attack%20Cooldown) (Variables|DefaultMeleeAttack|GetdefaultAttackCooldown)))

(event EventIAPlayerRangedAttack-Start
  ;[1 1 1] Ranged Attack
  (if (not (Variables|RangedMeleeAttack|GetrangedAttackCooldown))
    (Variables|RangedMeleeAttack|SetrangedAttackCooldown true)
    (Variables|RangedMeleeAttack|SetisCurrentlyRangedAttacking true)
    (Animation|Montage|PlayMontage (Variables|Character|GetMesh) "/Game/Animation/Player/Attack/Ranged/AM_ranged_attack.AM_ranged_attack"
      (:OnInterrupted
        (if (Variables|RangedMeleeAttack|GetisCurrentlyRangedAttacking)
          (Utilities|Time|SetTimerbyEvent (delegate Custom|Ranged%20Attack%20Cooldown%20End) (Variables|RangedMeleeAttack|GetrangedAttackCooldownLength) :!label _label)
          (Variables|RangedMeleeAttack|SetisCurrentlyRangedAttacking false)))
      (:OnNotifyBegin
        (Development|PrintString "Ranged")
        (CallFunction|SpawnRangedProjectile)
        (goto _label)))))

(event EventIAPlayerDefaultAttack-Start
  ;[1 1 1] Default Attack
  (if (not (and (Variables|DefaultMeleeAttack|GetdefaultMeleeCooldown) (not (Variables|RangedMeleeAttack|GetisCurrentlyRangedAttacking))))
    (if (not (Animation|Montage|MontageIsPlaying (Components|SkeletalMesh|GetAnimInstance (Variables|Character|GetMesh)) "/Game/Animation/Player/Attack/Default/AM_attack_combo.AM_attack_combo"))
      (Animation|Montage|PlayMontage (Variables|Character|GetMesh) "/Game/Animation/Player/Attack/Default/AM_attack_combo.AM_attack_combo"
        (:OnNotifyBegin
          (Variables|DefaultMeleeAttack|SetcomboWindow true)
          (Development|PrintString "COMBO WINDOW" true true "(R=1.000000,G=0.243137,B=0.529412,A=1.000000)"))
        (:OnNotifyEnd
          (bind _result (Math|Integer|DecrementInt (Variables|DefaultMeleeAttack|GetattackComboIndex))
            (:%20%20
              (if (< _result 0)
                (Animation|Montage|MontageStop (Components|SkeletalMesh|GetAnimInstance (Variables|Character|GetMesh)) 0.0 0)
                (Variables|DefaultMeleeAttack|SetattackComboIndex 0)
                (Utilities|FlowControl|Sequence
                  (:then_0
                    (Development|PrintString "END COMBO WINDOW" true true "(R=1.000000,G=0.243137,B=0.529412,A=1.000000)")
                    (Variables|DefaultMeleeAttack|SetcomboWindow false :!label _label))
                  (:then_1
                    (Variables|DefaultMeleeAttack|SetdefaultMeleeCooldown true)
                    (Utilities|Time|SetTimerbyEvent (delegate Custom|Disable%20Default%20Melee%20Attack%20Cooldown) (Variables|DefaultMeleeAttack|GetdefaultAttackCooldown))))
                (else
                  (goto _label)))))))
      (elif (Variables|DefaultMeleeAttack|GetcomboWindow)
        (Variables|DefaultMeleeAttack|SetattackComboIndex 1)))))

(event EventIAPlayerSprint-End)

(event EventEnableDefaultMeleeAttackTick
  ;[1 1 1] Default Attack
  (Utilities|Time|UnpauseTimerbyHandle (Variables|DefaultMeleeAttack|GetattackCkeckTickTimer))
  (Collision|SetCollisionEnabled (Variables|Default|GetCapsule) "QueryOnly"))

(event EventDisableDefaultMeleeAttackTick
  ;[1 1 1] Default Attack
  (Utilities|Time|PauseTimerbyHandle (Variables|DefaultMeleeAttack|GetattackCkeckTickTimer))
  (Collision|SetCollisionEnabled (Variables|Default|GetCapsule) "NoCollision"))

(event EventIAPlayerSprint-Start)

(event EventIAPlayerJump-End)

(event EventIAPlayerJump
  (Character|Jump))

(event EventIAPlayerLook
  (params (x :type Float%20%28double-precision%29) (y :type Float%20%28double-precision%29))
  (bind _mesh (Variables|Character|GetMesh))
  (bind _returnvalue (Components|SkeletalMesh|GetAnimInstance _mesh))
  (Utilities|FlowControl|Sequence
    (:then_0
      (Utilities|PlayerLook x y :!label _label))
    (:then_1
      (goto _label exec2))
    (:then_2
      (Class|BPIPlayerAnimation|Set"torsoRotationOverrideX"(Message) _returnvalue (.Yaw (Math|Rotator|BreakRotator (Pawn|GetControlRotation :!class /Script/Engine.Pawn))))
      (Class|BPIPlayerAnimation|Set"torsoRotationOverrideY"(Message) _returnvalue (.pitch (Transformation|GetWorldRotation (Variables|Default|GetCamera))))
      (Transformation|SetWorldLocation (Variables|Default|GetHead%20Hook) (Transformation|GetSocketLocation (Variables|Character|GetMesh) "Neck_01") false false))))

(event EventIAPlayerInspect-Start
  (Components|Animation|PlayAnimation (Variables|Character|GetMesh) (Variables|Default|GetinspectAnimation) false))

(event EventIAPlayerMovement
  (params (x :type Float%20%28double-precision%29) (y :type Float%20%28double-precision%29))
  (bind _returnvalue (Pawn|GetControlRotation :!class /Script/Engine.Pawn))
  (bind _mesh (Variables|Character|GetMesh))
  (bind _returnvalue_2 (Components|SkeletalMesh|GetAnimInstance _mesh))
  (Utilities|FlowControl|Sequence
    (:then_0
      (Pawn|Input|AddMovementInput (Math|Vector|GetForwardVector (Math|Rotator|MakeRotator 0.0 0.0 (.yaw _returnvalue))) y false))
    (:then_1
      (Pawn|Input|AddMovementInput (Math|Vector|GetRightVector (Math|Rotator|MakeRotator (.roll _returnvalue) 0.0 (.yaw _returnvalue))) x false)
      ;[1 0.5573 0.5573] Change Later
      (Class|PlayerController|SetMouseLocation (Game|GetPlayerController 0) 20 20))
    (:then_2
      (Class|BPIPlayerAnimation|Set"dir"(Message) _returnvalue_2 (Class|KismetMathLibrary|ClampAxis (Utilities|WalkDirectionCalculation x y)))
      (Class|BPIPlayerAnimation|Set"speed"(Message) _returnvalue_2 5e+01))))

(event EventTick
  (params (DeltaSeconds :type Float%20%28single-precision%29))
  (bind _flame (Variables|Default|GetFlame))
  (bind _flame_2 (Variables|Default|GetFlame))
  (bind _flamingswordfiregravityscaler (Variables|Default|GetflamingSwordFireGravityScaler))
  (bind _returnvalue (Transformation|GetWorldRotation _flame))
  (bind _returnvalue_2 (Math|Vector|GetUpVector _returnvalue))
  (bind _returnvalue_3 (* _returnvalue_2 _flamingswordfiregravityscaler))
  (Effects|Components|ParticleSystem|SetVectorParameter _flame_2 "referenceGravity" _returnvalue_3)
  (Effects|Components|ParticleSystem|SetVectorParameter _flame_2 "flameGravity" (* _returnvalue_3 (Math|Float|MakeLiteralFloat -1.0))))

(event EventIAPlayerMovement-End
  (Class|BPIPlayerAnimation|Set"speed"(Message) (Components|SkeletalMesh|GetAnimInstance (Variables|Character|GetMesh)) 0.0))

(fn ConstructionScript)

(fn AttackCheckRay
  (params (additionalRangeModif :type Float%20%28double-precision%29))
  (Development|PrintString (Utilities|String|ToString(Vector) (Transformation|GetSocketLocation (Variables|Character|GetMesh) "Hand_R")))
  (bind (_outhit _returnvalue) (Collision|SphereTraceForObjects (Transformation|GetWorldLocation (Variables|Default|GetBlade%20Base)) (Transformation|GetWorldLocation (Variables|Default|GetHit%20Range)) 1e+01 (Utilities|Array|MakeArray "ObjectTypeQuery7") false 0 "Persistent"))
  (return _returnvalue (.HitActor (Collision|BreakHitResult _outhit))))