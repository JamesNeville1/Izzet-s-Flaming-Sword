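; First-person player character with a visible body: it hides the head bone and pitches an orbiting camera hook so the player can see their feet.
; Input drives look, movement and jump, sending torso rotation, walk direction and speed to the animation instance.
; Inspect plays an animation and attack plays a combo montage with only a debug notify; sprint is stubbed.
; Tick feeds opposing gravity vectors, based on the flame's up vector, to the flaming sword effect.
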(event Custom|Start
  (Components|SkinnedMesh|HideBonebyName (Variables|Character|GetMesh) "head" "PBO_None"))

(event EventShouldCombo)

(event EventIAPlayerSprint-End)

(event EventIAPlayerDefaultAttack-Start
  (Animation|Montage|PlayMontage (Variables|Character|GetMesh) "/Game/Animation/Player/AM_attack_combo.AM_attack_combo"
    (:OnNotifyBegin
      (Development|PrintString "q"))))

(event EventIAPlayerSprint-Start)

(event EventIAPlayerJump-End)

(event EventIAPlayerJump
  (Character|Jump))

(event EventIAPlayerLook
  (params (x :type Float%20%28double-precision%29) (y :type Float%20%28double-precision%29))
  (Utilities|FlowControl|Sequence
    (:then_0
      (Pawn|Input|AddControllerYawInput (* x (Variables|Default|GetcameraSensitivity) -1.0)))
    (:then_1
      (Transformation|SetRelativeRotation (Variables|Default|GetCamera%20Hook) (Math|Rotator|MakeRotator (Math|Float|Clamp(Float) (+ (* y (Variables|Default|GetcameraSensitivity) -1.0) (.roll (Variables|/Script/Engine.SceneComponent|GetRelativeRotation (Variables|Default|GetCamera%20Hook)))) -8e+01 8e+01) 0.0 0.0) false false))
    (:then_2
      (Class|BPIPlayerAnimation|Set"torsoRotationOverride"(Message) (Components|SkeletalMesh|GetAnimInstance (Variables|Character|GetMesh)) (.Yaw (Math|Rotator|BreakRotator (Pawn|GetControlRotation :!class /Script/Engine.Pawn)))))))

(event EventIAPlayerInspect-Start
  (Components|Animation|PlayAnimation (Variables|Character|GetMesh) (Variables|Default|GetinspectAnimation) false))

(event EventIAPlayerMovement
  (params (x :type Float%20%28double-precision%29) (y :type Float%20%28double-precision%29))
  (bind _returnvalue (Pawn|GetControlRotation :!class /Script/Engine.Pawn))
  (bind _mesh (Variables|Character|GetMesh))
  (bind _returnvalue_2 (Components|SkeletalMesh|GetAnimInstance _mesh))
  (Utilities|FlowControl|Sequence
    (:then_0
      (Pawn|Input|AddMovementInput (Math|Vector|GetForwardVector (Math|Rotator|MakeRotator 0.0 0.0 (.yaw _returnvalue))) y false))
    (:then_1
      (Pawn|Input|AddMovementInput (Math|Vector|GetRightVector (Math|Rotator|MakeRotator (.roll _returnvalue) 0.0 (.yaw _returnvalue))) x false)
      ;[1 0.5573 0.5573] Change Later
      (Class|PlayerController|SetMouseLocation (Game|GetPlayerController 0) 20 20))
    (:then_2
      (Class|BPIPlayerAnimation|Set"dir"(Message) _returnvalue_2 (Class|KismetMathLibrary|ClampAxis (Utilities|WalkDirectionCalculation x y)))
      (Class|BPIPlayerAnimation|Set"speed"(Message) _returnvalue_2 5e+01))))

(event EventTick
  (params (DeltaSeconds :type Float%20%28single-precision%29))
  (bind _flame (Variables|Default|GetFlame))
  (bind _flame_2 (Variables|Default|GetFlame))
  (bind _flamingswordfiregravityscaler (Variables|Default|GetflamingSwordFireGravityScaler))
  (bind _returnvalue (Transformation|GetWorldRotation _flame))
  (bind _returnvalue_2 (Math|Vector|GetUpVector _returnvalue))
  (bind _returnvalue_3 (* _returnvalue_2 _flamingswordfiregravityscaler))
  (Effects|Components|ParticleSystem|SetVectorParameter _flame_2 "referenceGravity" _returnvalue_3)
  (Effects|Components|ParticleSystem|SetVectorParameter _flame_2 "flameGravity" (* _returnvalue_3 (Math|Float|MakeLiteralFloat -1.0))))

(event EventIAPlayerMovement-End
  (Class|BPIPlayerAnimation|Set"speed"(Message) (Components|SkeletalMesh|GetAnimInstance (Variables|Character|GetMesh)) 0.0))

(fn ConstructionScript)