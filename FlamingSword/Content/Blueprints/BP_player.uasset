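; BP_player is the player character, handling look, movement, jump and an inspect animation from Enhanced Input actions.
; Look input turns controller yaw, passes it to the mesh's anim instance, and rotates a clamped CameraHook so the player can see their feet.
; Movement follows control yaw and also resets the mouse position, marked as temporary.
; Sprint events are empty stubs, and a debug yaw print remains.
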(event Custom|Start)

(event EventIAPlayerMovement
  (params (x :type Float%20%28double-precision%29) (y :type Float%20%28double-precision%29))
  (bind _returnvalue (Pawn|GetControlRotation :!class /Script/Engine.Pawn))
  (Utilities|FlowControl|Sequence
    (:then_0
      (Pawn|Input|AddMovementInput (Math|Vector|GetForwardVector (Math|Rotator|MakeRotator 0.0 0.0 (.yaw _returnvalue))) y false))
    (:then_1
      (Pawn|Input|AddMovementInput (Math|Vector|GetRightVector (Math|Rotator|MakeRotator (.roll _returnvalue) 0.0 (.yaw _returnvalue))) x false)
      ;[1 0.5573 0.5573] Change Later
      (Class|PlayerController|SetMouseLocation (Game|GetPlayerController 0) 20 20))))

(event EventIAPlayerSprint-End)

(event EventIAPlayerSprint-Start)

(event EventIAPlayerJump-End)

(event EventIAPlayerJump
  (Character|Jump))

(event EventIAPlayerLook
  (params (x :type Float%20%28double-precision%29) (y :type Float%20%28double-precision%29))
  (bind _returnvalue (Pawn|GetControlRotation :!class /Script/Engine.Pawn))
  (Utilities|FlowControl|Sequence
    (:then_0
      (Pawn|Input|AddControllerYawInput (* x (Variables|Default|GetcameraSensitivity) -1.0))
      (Class|BPIPlayerAnimation|Set"dir"(Message) (Components|SkeletalMesh|GetAnimInstance (Variables|Character|GetMesh)) (.yaw _returnvalue))
      (Development|PrintString (Utilities|String|ToString(Float) (.yaw _returnvalue))))
    (:then_1
      (Transformation|SetRelativeRotation (Variables|Default|GetCamera%20Hook) (Math|Rotator|MakeRotator (Math|Float|Clamp(Float) (+ (* y (Variables|Default|GetcameraSensitivity) -1.0) (.roll (Variables|/Script/Engine.SceneComponent|GetRelativeRotation (Variables|Default|GetCamera%20Hook)))) -8e+01 8e+01) 0.0 0.0) false false))))

(event EventIAPlayerInspect-Start
  (Components|Animation|PlayAnimation (Variables|Character|GetMesh) (Variables|Default|GetinspectAnimation) false))

(fn ConstructionScript)